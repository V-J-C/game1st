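; Slot-based player inventory that adds, stacks, removes and uses items, exposes its data for saving, and sizes its slots only on a new game.
; Slots hold an item class and amount, with stacking rules read from class defaults.
; It creates a hidden widget on the main HUD, refreshes changed slots, and switches cursor and input mode on open/close.
; Using an item while open spawns its actor and calls UseItem.
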(event EventBeginPlay
  (switch Utilities|FlowControl|Switch|SwitchonE_InventoryStartMod (Variables|Default|GetStart%20Mod)
    (:NewEnumerator0
      (Utilities|Array|Resize (Variables|Default|GetSlots) (Variables|Default|GetAmountOfSlots))
      (CallFunction|CreateInventoryWidget))
    (:NewEnumerator1
      (CallFunction|CreateInventoryWidget))))

(fn ConstructionScript)

(fn GetSaveData
  (return (Utilities|Struct|MakeS_saveInventoryInfo (Variables|Default|GetAmountOfSlots) (Variables|Default|GetSlots))))

(fn GetSlotInfofromIndex
  (params (Index :type Integer))
  (bind _slots (Variables|Default|GetSlots))
  (bind _output (Utilities|Array|Get(acopy) _slots Index))
  (bind (_item _amount) (Utilities|Struct|BreakS_SlotSignature _output))
  ;[1 1 1] Проверяем на пустой слот
  (if (Utilities|IsValidClass _item)
    ;[0.2409 1 0.04797] Если не пустой, выводим сигеатуру
    (return false (.ItemSignature (Utilities|GetClassDefaults _item)) _amount)
    (else
      ;[1 0 0] Если слот пустой, Выдаем пустой слот
      (return true "" 0))))

(fn CreateInventoryWidget
  ;[1 1 1] Создаем виджет инвентаря и записываем его в переменную
  (bind _returnvalue (UserInterface|CreateWidget "/Game/Inventory/Widgets/Inv_WB.Inv_WB_C" 0 self))
  (bind _output_get (Variables|Default|SetInv_WB%20Ref _returnvalue))
  (Widget|SetVisibility _output_get "Hidden")
  ;[1 1 1] Добавляем воджет на экран
  (bind _returnvalue_2 (Class|CanvasPanel|AddChildtoCanvas (Variables|/Game/UI/HUD/Main_HUD.Main_HUD_C|GetCanvasPanel_0 (Variables|Default|GetMain%20HUD)) _output_get))
  (Class|CanvasPanelSlot|SetAutoSize _returnvalue_2 true)
  (Class|CanvasPanelSlot|SetPosition _returnvalue_2 (/ (Viewport|GetViewportSize) "(X=1.300000,Y=2.000000)"))
  (return))

(fn ShowInventory
  (bind _returnvalue (Game|GetPlayerController 0))
  (Utilities|IsValid (Variables|Default|GetInv_WB%20Ref)
    (:Is%20Valid
      ;[1 1 1] Проверка статуса инвенторя
      (switch Utilities|FlowControl|Switch|SwitchonE_InventoryStatus (Variables|Default|GetStatus)
        (:NewEnumerator0
          (Widget|SetVisibility (Variables|Default|GetInv_WB%20Ref) "Visible")
          ;[1 1 1] Включаем мышку и фокус на виджет
          (Variables|/Script/Engine.PlayerController|SetbShowMouseCursor _returnvalue true)
          (Input|SetInputModeGameandUI _returnvalue (Variables|Default|GetMain%20HUD) "DoNotLock" false)
          (Variables|Default|SetStatus "NewEnumerator1")
          (return))))))

(fn HideInventory
  (bind _returnvalue (Game|GetPlayerController 0))
  (Utilities|IsValid (Variables|Default|GetInv_WB%20Ref)
    (:Is%20Valid
      ;[1 1 1] Проверка статуса инвентаря
      (switch Utilities|FlowControl|Switch|SwitchonE_InventoryStatus (Variables|Default|GetStatus)
        (:NewEnumerator1
          (Widget|SetVisibility (Variables|Default|GetInv_WB%20Ref) "Hidden")
          ;[1 1 1] Убираем курсор мышки и ставим фокус на игру
          (Variables|/Script/Engine.PlayerController|SetbShowMouseCursor _returnvalue false)
          (Input|SetInputModeGameOnly _returnvalue)
          (Variables|Default|SetStatus "NewEnumerator0")
          (return))))))

(fn HideShowInventoryFlipFlop
  (switch Utilities|FlowControl|Switch|SwitchonE_InventoryStatus (Variables|Default|GetStatus)
    (:NewEnumerator0
      (HideShowInventory|ShowInventory))
    (:NewEnumerator1
      (HideShowInventory|HideInventory))))

(fn UpdateWidgetSlot
  (params (Ibdex :type Integer))
  (Default|UpdateSlot (Utilities|Array|Get(acopy) (Variables|/Game/Inventory/Widgets/Inv_WB.Inv_WB_C|GetSlot%20widgets%20Array (Variables|Default|GetInv_WB%20Ref)) Ibdex)))

(fn SeartchAnAmptySlot
  (bind (_array_element _array_index) (Utilities|Array|ForEachLoopwithBreak (Variables|Default|GetSlots) :!label _label)
    (:LoopBody
      (if (not (Utilities|IsValidClass (.Item (Utilities|Struct|BreakS_SlotSignature _array_element))))
        (LocalVariables|SetLocal%20Boolean true)
        (LocalVariables|SetLocal%20Index _array_index)
        (goto _label Break)))
    (:Completed
      (return (LocalVariables|GetLocal%20Boolean) (LocalVariables|GetLocal%20Index)))))

(fn SearchSlotIndexforStack
  (params (Item :type BP%20Master%20Item%20Class%20Reference))
  (bind (_array_element _array_index) (Utilities|Array|ForEachLoopwithBreak (Variables|Default|GetSlots) :!label _label)
    (:LoopBody
      (if (and (Utilities|IsValidClass (.Item (Utilities|Struct|BreakS_SlotSignature _array_element))) (== (.Item (Utilities|Struct|BreakS_SlotSignature _array_element)) Item))
        (LocalVariables|SetLocal%20Steck%20is%20Founded true)
        (goto _label Break)))
    (:Completed
      (return (LocalVariables|GetLocal%20Steck%20is%20Founded) _array_index))))

(fn AddItem
  (params (Iyem :type BP%20Master%20Item%20Class%20Reference) (Amount :type Integer))
  (bind _slots (Variables|Default|GetSlots))
  (LocalVariables|SetLocal%20Item Iyem)
  (bind _output_get (LocalVariables|SetLocal%20amount Amount))
  ;[1 1 1] проверка на 0 кол-во итемов
  (if (> _output_get 0)
    ;[1 1 1] Проверка стакается ли предмет
    (if (.stackable (.ItemSignature (Utilities|GetClassDefaults (LocalVariables|GetLocal%20Item))))
      ;[1 1 1] Ищим есть ли куда пристакать итем или нужно добавить новый слот
      (bind (_seccsess _founded_index) (CallFunction|SearchSlotIndexforStack (LocalVariables|GetLocal%20Item)))
      (if _seccsess
        ;[1 1 1] Если итем стакается и уже есть такой же придмет , тогда пристакиваеи
        ;;[1 1 1] Стакаем кол-во итемов в один слот
        (Utilities|Array|SetArrayElem _slots _founded_index (Utilities|Struct|MakeS_SlotSignature (LocalVariables|GetLocal%20Item) (+ (.amount (Utilities|Array|Get(acopy) _slots _founded_index)) (LocalVariables|GetLocal%20amount))))
        ;;[1 1 1] Обновляем виджет
        (CallFunction|UpdateWidgetSlot _founded_index)
        ;;[0 1 0] Предмет Пристакан
        (return true "NewEnumerator1")
        (else
          _)))
    ;[1 1 1] Если предмет не стакается или нет предмета к которому можно пристакать тогда добовляем новый предмет в новый слот
    ;;[1 1 1] Ищем пустой слот, если не находим-> ошибка
    (bind (_success _index) (CallFunction|SeartchAnAmptySlot))
    (if _success
      ;;[1 1 1] Добовляем придмет в инвентарь
      (Utilities|Array|SetArrayElem (Variables|Default|GetSlots) _index (Utilities|Struct|MakeS_SlotSignature (LocalVariables|GetLocal%20Item) (LocalVariables|GetLocal%20amount)))
      ;;[1 1 1] Обновляем виджет
      (CallFunction|UpdateWidgetSlot _index)
      ;;[0 1 0] Предмет добавлен
      (return true "NewEnumerator0")
      (else
        ;;[1 0 0] Ошибка: Нету места в инвентаре
        (return false "NewEnumerator2")))))

(fn RemoveItematIndex
  (params (Index :type Integer) (Amount :type Integer))
  (bind _slots (Variables|Default|GetSlots))
  (LocalVariables|SetLocalIndex Index)
  (LocalVariables|SetLocalAmount Amount)
  ;[1 1 1] Является ли колличество удл итемов  больше чем кол-во итемов в слоте
  (if (>= (LocalVariables|GetLocalAmount) (.Amount (CallFunction|GetSlotInfofromIndex (LocalVariables|GetLocalIndex))))
    ;[1 1 1] Удаляем весь слот
    (Utilities|Array|SetArrayElem (Variables|Default|GetSlots) (LocalVariables|GetLocalIndex) (Utilities|Struct|MakeS_SlotSignature 0 0))
    ;[1 1 1] Обновляем виджет слотов
    (CallFunction|UpdateWidgetSlot (LocalVariables|GetLocalIndex))
    (return)
    (else
      ;[1 1 1] Удаляем Колличество слот
      (Utilities|Array|SetArrayElem _slots (LocalVariables|GetLocalIndex) (Utilities|Struct|MakeS_SlotSignature (.item (Utilities|Array|Get(acopy) _slots (LocalVariables|GetLocalIndex))) (- (.amount (Utilities|Array|Get(acopy) _slots (LocalVariables|GetLocalIndex))) (LocalVariables|GetLocalAmount))))
      ;[1 1 1] Обновляем виджет слотов
      (CallFunction|UpdateWidgetSlot (LocalVariables|GetLocalIndex))
      (return))))

(fn UseItematIndex
  (params (Index :type Integer))
  (LocalVariables|SetLocalIndex Index)
  (switch Utilities|FlowControl|Switch|SwitchonE_InventoryStatus (Variables|Default|GetStatus)
    (:NewEnumerator1
      (bind _returnvalue (Game|SpawnActorfromClass (.item (Utilities|Array|Get(acopy) (Variables|Default|GetSlots) (LocalVariables|GetLocalIndex))) (Math|Transform|MakeTransform "0, 0, 0" "0, 0, 0" "1,1,1") "Undefined" 0 self (LocalVariables|GetLocalIndex) 0))
      (Default|UseItem _returnvalue))))