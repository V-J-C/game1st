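; World actor that represents an inventory item in the level, showing the item's mesh and a name widget.
; On BeginPlay it reads the ItemSignature from the class defaults of its Item class, so the item is not instantiated.
; That data sets the static mesh and feeds the WorldItem_WB widget the name and stackable flag, along with the actor's own Amount.
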(event EventBeginPlay
  ;[1 1 1] устанавливаем меш и название итема
  (CallFunction|Initialize3DMash)
  (CallFunction|InitializeItemName))

(fn ConstructionScript)

(fn Initialize3DMash
  (Components|StaticMesh|SetStaticMesh (Variables|Default|GetItemMash) (.3dmash (.ItemSignature (Utilities|GetClassDefaults (Variables|Default|GetItem))))))

(fn InitializeItemName
  (bind _item (Variables|Default|GetItem))
  (bind _itemsignature (Utilities|GetClassDefaults _item))
  (bind _asworld_item_wb (Utilities|Casting|CastToWorldItem_WB (UserInterface|GetUserWidgetObject (Variables|Default|GetWidget))))
  (Default|SetItemName _asworld_item_wb (.name _itemsignature) (.stackable _itemsignature) (Variables|Default|GetAmount)))